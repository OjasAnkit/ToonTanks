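; BP_PawnTurret is a turret pawn that shows an enemy health widget while a player tank is nearby.
; On BeginPlay it caches the HealthWidget component's user widget as a WBP_HealthEnemy reference.
; Overlap events on UIShowUpRadius toggle the widget's visibility when a BP_PawnTank enters or leaves.
; The graph never updates the health value, as its only HealthOfTurret setter is unconnected.
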(event OnComponentBeginOverlap(UIShowupradius)
  (params (OverlappedComponent :type Primitive%20Component%20Object%20Reference) (OtherActor :type Actor%20Object%20Reference) (OtherComp :type Primitive%20Component%20Object%20Reference) (OtherBodyIndex :type Integer) (bFromSweep :type Boolean) (SweepResult :type Hit%20Result%20Structure%20%28by%20ref%29))
  (Utilities|Casting|CastToBP_PawnTank OtherActor)
  (Rendering|SetVisibility (Variables|Default|GetHealthWidget) true false))

(event OnComponentEndOverlap(UIShowupradius)
  (params (OverlappedComponent :type Primitive%20Component%20Object%20Reference) (OtherActor :type Actor%20Object%20Reference) (OtherComp :type Primitive%20Component%20Object%20Reference) (OtherBodyIndex :type Integer))
  (Utilities|Casting|CastToBP_PawnTank OtherActor)
  (Rendering|SetVisibility (Variables|Default|GetHealthWidget) false false))

(event EventBeginPlay
  (bind _aswbp_health_enemy (Utilities|Casting|CastToWBP_HealthEnemy (UserInterface|GetUserWidgetObject (Variables|Default|GetHealthWidget))))
  (Variables|Default|SetHealthWidgetRef _aswbp_health_enemy))

(event Collision|EventActorBeginOverlap
  (params (OtherActor :type Actor%20Object%20Reference)))

(event EventTick
  (params (DeltaSeconds :type Float%20%28single-precision%29)))

(fn ConstructionScript)